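; Moving sprite Blueprint that sends a magic torch-fire effect gliding along a spline when something enters its trigger box.
; Any overlap with ActiveBox calls Move, which plays MoveTimeline at a rate set by Speed.
; The timeline track maps to distance along the spline, moving NSTorchFireMagic to that world position each update.
; The effect deactivates when the timeline finishes, and nothing reactivates or rewinds it.
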(event `self.ReceiveBeginPlay`)

(event `Move`
  (`TimelineComponent.SetPlayRate` (`self.MoveTimeline`) (`self.Speed`))
  (bind (_direction _movetrack) (`Timeline|MoveTimeline`)
    (:`Update`
      (bind _returnvalue_location (`KismetMathLibrary.BreakTransform` (`SplineComponent.GetTransformAtDistanceAlongSpline` (`self.Spline`) (`KismetMathLibrary.Lerp` 0.0 (`SplineComponent.GetSplineLength` (`self.Spline`)) _movetrack) "World" false)))
      (`SceneComponent.K2_SetWorldLocationAndRotation` :`self` (`self.NS_TorchFire_Magic`) :`NewLocation` _returnvalue_location))
    (:`Finished`
      (`ActorComponent.Deactivate` (`self.NS_TorchFire_Magic`)))))

(event `self.ActiveBox.OnComponentBeginOverlap`
  (params (OverlappedComponent :type "PrimitiveComponent Object Reference") (OtherActor :type "Actor Object Reference") (OtherComp :type "PrimitiveComponent Object Reference") (OtherBodyIndex :type Integer) (bFromSweep :type Boolean) (SweepResult :type "HitResult Structure (by ref)"))
  (`self.Move`))

(fn `UserConstructionScript`)